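; Spider enemy actor that bites the VR player pawn and dies when hit by an arrow projectile.
; Overlapping the attack area sets an attack flag, applies damage once and plays a random attack sound; leaving clears the flag.
; An arrow entering the hit volume sets the dead flag, plays a death sound, then after a short delay spawns Exp_arrow and destroys the spider.
; ShowLight is hidden shortly after BeginPlay.
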(event OnComponentBeginOverlap(Attact_area)
  (params (OverlappedComponent :type Primitive%20Component%20Object%20Reference) (OtherActor :type Actor%20Object%20Reference) (OtherComp :type Primitive%20Component%20Object%20Reference) (OtherBodyIndex :type Integer) (bFromSweep :type Boolean) (SweepResult :type Hit%20Result%20Structure%20%28by%20ref%29))
  (bind _returnvalue (Transformation|GetActorLocation))
  (Utilities|Casting|CastToVive_PawnCharacter OtherActor)
  (Variables|Default|SetIs_attack true)
  (Game|Damage|ApplyDamage 0 1e+01 0 0 "/Script/Engine.DamageType")
  (bind _output_get (Variables|Default|Setselect_sound (Math|Random|RandomInteger 3)))
  (switch int _output_get
    (:0
      (Audio|PlaySoundatLocation "/Game/Enemy/Spider/Spider_sound/Spider_attack1.Spider_attack1" _returnvalue "0, 0, 0" 1.0 1.0 0.0 0 0 0))
    (:1
      (Audio|PlaySoundatLocation "/Game/Enemy/Spider/Spider_sound/Spider_attack2.Spider_attack2" _returnvalue "0, 0, 0" 1.0 1.0 0.0 0 0 0))
    (:2
      (Audio|PlaySoundatLocation "/Game/Enemy/Spider/Spider_sound/Spider_attack2.Spider_attack2" _returnvalue "0, 0, 0" 1.0 1.0 0.0 0 0 0))
    (:3
      (Audio|PlaySoundatLocation "/Game/Enemy/Spider/Spider_sound/Spider_attack4.Spider_attack4" _returnvalue "0, 0, 0" 1.0 1.0 0.0 0 0 0))))

(event OnComponentEndOverlap(Attact_area)
  (params (OverlappedComponent :type Primitive%20Component%20Object%20Reference) (OtherActor :type Actor%20Object%20Reference) (OtherComp :type Primitive%20Component%20Object%20Reference) (OtherBodyIndex :type Integer))
  (Utilities|Casting|CastToVive_PawnCharacter OtherActor)
  (Variables|Default|SetIs_attack false))

(event OnComponentBeginOverlap(Get_Attack)
  (params (OverlappedComponent :type Primitive%20Component%20Object%20Reference) (OtherActor :type Actor%20Object%20Reference) (OtherComp :type Primitive%20Component%20Object%20Reference) (OtherBodyIndex :type Integer) (bFromSweep :type Boolean) (SweepResult :type Hit%20Result%20Structure%20%28by%20ref%29))
  (Utilities|Casting|CastToArrow_Projectile OtherActor)
  (Variables|Default|SetBP_Is_dead true)
  (Audio|PlaySoundatLocation "/Game/Enemy/Spider/Spider_sound/Spider_dead.Spider_dead" (Transformation|GetActorLocation) "0, 0, 0" 1.0 1.0 0.0 0 0 0)
  (Utilities|FlowControl|Delay 0.9)
  (Game|SpawnActorfromClass "/Game/VRWapen/Arrow/Exp_arrow.Exp_arrow_C" (Math|Conversions|ToTransform(Vector) (Transformation|GetActorLocation)) "Undefined" 0 0)
  (Actor|DestroyActor))

(event EventBeginPlay
  (Utilities|FlowControl|Delay 2.0)
  (Development|SetHiddeninGame (Variables|Default|GetShow_light) true false))

(fn ConstructionScript)