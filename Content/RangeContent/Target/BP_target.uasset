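; Archery target Blueprint that scores arrow hits on yellow, red and blue zones.
; Each zone's overlap filters for Arrow_Projectile, plays its own sound and adds its point value to Score, with yellow highest.
; All zones then share a path that prints Score and, at the threshold, spawns what comments call an elevator at a hardcoded transform.
; The spawn has no once-only guard, so it repeats on later hits.
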(event OnComponentBeginOverlap(blue)
  (params (OverlappedComponent :type Primitive%20Component%20Object%20Reference) (OtherActor :type Actor%20Object%20Reference) (OtherComp :type Primitive%20Component%20Object%20Reference) (OtherBodyIndex :type Integer) (bFromSweep :type Boolean) (SweepResult :type Hit%20Result%20Structure%20%28by%20ref%29))
  ;[1 1 1] Detect arrow overlap and play sound effect
  (Utilities|Casting|CastToArrow_Projectile OtherActor)
  (Audio|PlaySoundatLocation "/Game/RangeContent/Target/target_sound/Arrow_on_target3.Arrow_on_target3" (Transformation|GetActorLocation) "0, 0, 0" 1.0 1.0 0.0 0 0 0)
  ;[1 1 1] Adding point
  (bind _output_get (Variables|Default|Settmp_num_blue 20))
  (Variables|Default|Setscore (+ (Variables|Default|Getscore) _output_get))
  (Development|PrintString (Utilities|String|ToString(Integer) (Variables|Default|Getscore)))
  ;[1 1 1] Spawn elevator at 500 point
  (if (<= 500 (Variables|Default|Getscore))
    (Game|SpawnActorfromClass "/Game/RangeContent/Elevator/Go_Desert.Go_Desert_C" (Math|Transform|MakeTransform "-1220.000000,3510.000000,280.000000" "0, 0, 0" "2.000000,2.000000,2.000000") "Undefined" 0 0)))

(event OnComponentBeginOverlap(yellow)
  (params (OverlappedComponent :type Primitive%20Component%20Object%20Reference) (OtherActor :type Actor%20Object%20Reference) (OtherComp :type Primitive%20Component%20Object%20Reference) (OtherBodyIndex :type Integer) (bFromSweep :type Boolean) (SweepResult :type Hit%20Result%20Structure%20%28by%20ref%29))
  ;[1 1 1] Detect arrow overlap and play sound effect
  (Utilities|Casting|CastToArrow_Projectile OtherActor)
  (Audio|PlaySoundatLocation "/Game/RangeContent/Target/target_sound/Arrow_on_target1.Arrow_on_target1" (Transformation|GetActorLocation) "0, 0, 0" 1.0 1.0 0.0 0 0 0)
  ;[1 1 1] Adding point
  (bind _output_get (Variables|Default|Settmp_num_yellow 100))
  (Variables|Default|Setscore (+ (Variables|Default|Getscore) _output_get))
  (Development|PrintString (Utilities|String|ToString(Integer) (Variables|Default|Getscore)))
  ;[1 1 1] Spawn elevator at 500 point
  (if (<= 500 (Variables|Default|Getscore))
    (Game|SpawnActorfromClass "/Game/RangeContent/Elevator/Go_Desert.Go_Desert_C" (Math|Transform|MakeTransform "-1220.000000,3510.000000,280.000000" "0, 0, 0" "2.000000,2.000000,2.000000") "Undefined" 0 0)))

(event OnComponentBeginOverlap(red)
  (params (OverlappedComponent :type Primitive%20Component%20Object%20Reference) (OtherActor :type Actor%20Object%20Reference) (OtherComp :type Primitive%20Component%20Object%20Reference) (OtherBodyIndex :type Integer) (bFromSweep :type Boolean) (SweepResult :type Hit%20Result%20Structure%20%28by%20ref%29))
  ;[1 1 1] Detect arrow overlap and play sound effect
  (Utilities|Casting|CastToArrow_Projectile OtherActor)
  (Audio|PlaySoundatLocation "/Game/RangeContent/Target/target_sound/Arrow_on_target2.Arrow_on_target2" (Transformation|GetActorLocation) "0, 0, 0" 1.0 1.0 0.0 0 0 0)
  ;[1 1 1] Adding point
  (bind _output_get (Variables|Default|Settmp_num_red 50))
  (Variables|Default|Setscore (+ (Variables|Default|Getscore) _output_get))
  (Development|PrintString (Utilities|String|ToString(Integer) (Variables|Default|Getscore)))
  ;[1 1 1] Spawn elevator at 500 point
  (if (<= 500 (Variables|Default|Getscore))
    (Game|SpawnActorfromClass "/Game/RangeContent/Elevator/Go_Desert.Go_Desert_C" (Math|Transform|MakeTransform "-1220.000000,3510.000000,280.000000" "0, 0, 0" "2.000000,2.000000,2.000000") "Undefined" 0 0)))

(fn ConstructionScript)