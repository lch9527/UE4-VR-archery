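; VR bow that nocks normal or explosive arrows and fires them from a string slider.
; Overlapping the Attach component with an arrow actor destroys it, sets its on-string flag and shows a stand-in arrow mesh, plus fire for explosive arrows.
; Dropping the string reads and resets slider progress after a brief delay, then spawns the matching projectile, launched forward with speed scaled by draw.
; Only normal shots play the release sound.
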(event OnDropped(String_slider)
  (params (GrippingController :type Grip%20Motion%20Controller%20Component%20Object%20Reference) (GripInformation :type BP%20Actor%20Grip%20Information%20Structure%20%28by%20ref%29) (bWasSocketed :type Boolean))
  (bind _arrow_transform (Variables|Default|GetArrow_Transform))
  (bind _arrow_transform_2 (Variables|Default|GetArrow_Transform))
  (bind _string_slider (Variables|Default|GetString_slider))
  (bind _returnvalue (Transformation|GetWorldTransform _arrow_transform))
  (bind _returnvalue_2 (Math|Vector|GetForwardVector _arrow_transform_2))
  (Utilities|FlowControl|Delay 0.1)
  (Variables|Default|SetSliderProgress (Variables|/Script/VRExpansionPlugin.VRSliderComponent|GetCurrentSliderProgress _string_slider))
  (Class|VRSliderComponent|SetSliderProgress _string_slider 0.0)
  (if (Variables|Default|GetArrowOnstring)
    (bind _returnvalue_3 (Game|SpawnActorfromClass "/Game/VRWapen/Arrow/Arrow_Projectile.Arrow_Projectile_C" _returnvalue "Undefined" 0 0))
    (Audio|PlaySoundatLocation "/Game/VRWapen/Bs_bow/Sound_effect/bow_release.bow_release" "0, 0, 0" "0, 0, 0" 1.0 1.0 0.0 0 0 0)
    (Variables|Default|SetArrowOnstring false)
    (Default|Arrowspeed _returnvalue_3 (+ (* (Variables|Default|GetSliderProgress) 3e+03) 1.0) _returnvalue_2)
    (Development|SetHiddeninGame (Variables|Default|GetArrow_mesh) true false)
    (elif (Variables|Default|GetExpArrowOnstring)
      (bind _returnvalue_4 (Game|SpawnActorfromClass "/Game/VRWapen/Arrow/Exp_Arrow_projectile.Exp_Arrow_projectile_C" _returnvalue "Undefined" 0 0))
      (Variables|Default|SetExpArrowOnstring false)
      (Default|Arrowspeed _returnvalue_4 (+ (* (Variables|Default|GetSliderProgress) 3e+03) 1.0) _returnvalue_2)
      (Development|SetHiddeninGame (Variables|Default|GetArrow_mesh) true false)
      (Development|SetHiddeninGame (Variables|Default|Getfire) true false))))

(event OnComponentBeginOverlap(Attach)
  (params (OverlappedComponent :type Primitive%20Component%20Object%20Reference) (OtherActor :type Actor%20Object%20Reference) (OtherComp :type Primitive%20Component%20Object%20Reference) (OtherBodyIndex :type Integer) (bFromSweep :type Boolean) (SweepResult :type Hit%20Result%20Structure%20%28by%20ref%29))
  (bind _asbp_arrow (Utilities|Casting|CastToBP_arrow OtherActor)
    (:then
      (Variables|Default|SetArrowOnstring true)
      (Actor|DestroyActor _asbp_arrow))
    (:CastFailed
      (bind _asexp_arrow (Utilities|Casting|CastToExp_arrow OtherActor))
      (Variables|Default|SetExpArrowOnstring true)
      (Development|SetHiddeninGame (Variables|Default|Getfire) false false)
      (Actor|DestroyActor _asexp_arrow)))
  (Development|SetHiddeninGame (Variables|Default|GetArrow_mesh) false false))

(fn ConstructionScript)