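; VR bow actor that nocks and fires normal or explosive arrows.
; Overlapping the Attach component with a held arrow destroys it, flags its type and shows a stand-in mesh on the bow.
; Dropping the string slider saves the pull amount after a short delay, resets the string and spawns the matching projectile with speed scaled by pull.
; An empty release only plays a half-release sound.
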(event OnComponentBeginOverlap(Attach)
  (params (OverlappedComponent :type Primitive%20Component%20Object%20Reference) (OtherActor :type Actor%20Object%20Reference) (OtherComp :type Primitive%20Component%20Object%20Reference) (OtherBodyIndex :type Integer) (bFromSweep :type Boolean) (SweepResult :type Hit%20Result%20Structure%20%28by%20ref%29))
  ;[1 1 1] detect is an arrow on the string and destroy the arrow on player's hand
  (bind _asbp_arrow (Utilities|Casting|CastToBP_arrow OtherActor)
    (:then
      (Variables|Default|SetArrowOnstring true)
      (Actor|DestroyActor _asbp_arrow))
    (:CastFailed
      (bind _asexp_arrow (Utilities|Casting|CastToExp_arrow OtherActor))
      (Variables|Default|SetExpArrowOnstring true)
      (Actor|DestroyActor _asexp_arrow)))
  ;[1 1 1] Set arrow visable on the bow
  (Development|SetHiddeninGame (Variables|Default|GetArrow_mesh) false false))

(event OnDropped(SF_string)
  (params (GrippingController :type Grip%20Motion%20Controller%20Component%20Object%20Reference) (GripInformation :type BP%20Actor%20Grip%20Information%20Structure%20%28by%20ref%29) (bWasSocketed :type Boolean))
  (bind _arrow_transform (Variables|Default|GetArrow_Transform))
  (bind _sf_string (Variables|Default|GetSF_string))
  (bind _arrow_transform_2 (Variables|Default|GetArrow_Transform))
  (bind _returnvalue (Transformation|GetWorldTransform _arrow_transform))
  (bind _returnvalue_2 (Math|Vector|GetForwardVector _arrow_transform_2))
  ;[1 1 1] When stringing release, Save the string-pulling to the viable sliderPorgress, and reset the string position to 0
  (Utilities|FlowControl|Delay 0.1)
  (Variables|Default|SetSliderProgress (Variables|/Script/VRExpansionPlugin.VRSliderComponent|GetCurrentSliderProgress _sf_string))
  (Class|VRSliderComponent|SetSliderProgress _sf_string 0.0)
  ;[1 1 1] detect is an arrow on the string and what kind of arrow is on the string
  (if (Variables|Default|GetArrowOnstring)
    ;[1 1 1] Spawn arrow Projectile depend on arrow type
    (bind _returnvalue_3 (Game|SpawnActorfromClass "/Game/VRWapen/Arrow/Arrow_Projectile.Arrow_Projectile_C" _returnvalue "Undefined" 0 0))
    ;[1 1 1] Sound effect for arrow
    (Audio|PlaySoundatLocation "/Game/VRWapen/SF_Bow/SF_Bow_sound/SF_full_release.SF_full_release" (Transformation|GetActorLocation) "0, 0, 0" 1.0 1.0 0.0 0 0 0)
    (Variables|Default|SetArrowOnstring false)
    ;[1 1 1] Set arrow speed depend on how far the player pull the string
    (Default|Arrowspeed _returnvalue_3 (+ (* (Variables|Default|GetSliderProgress) 6e+03) 1.0) _returnvalue_2)
    ;[1 1 1] Set arrow invisible after shooting
    (Development|SetHiddeninGame (Variables|Default|GetArrow_mesh) true false)
    (elif (Variables|Default|GetExpArrowOnstring)
      (bind _returnvalue_4 (Game|SpawnActorfromClass "/Game/VRWapen/Arrow/Exp_Arrow_projectile.Exp_Arrow_projectile_C" _returnvalue "Undefined" 0 0))
      ;[1 1 1] Sound effect for arrow
      (Audio|PlaySoundatLocation "/Game/VRWapen/SF_Bow/SF_Bow_sound/SF_full_release.SF_full_release" (Transformation|GetActorLocation) "0, 0, 0" 1.0 1.0 0.0 0 0 0)
      (Variables|Default|SetExpArrowOnstring false)
      (Default|Arrowspeed _returnvalue_4 (+ (* (Variables|Default|GetSliderProgress) 6e+03) 1.0) _returnvalue_2)
      (Development|SetHiddeninGame (Variables|Default|GetArrow_mesh) true false)
      (Development|SetHiddeninGame (Variables|Default|Getfire) true false)
      (else
        ;[1 1 1] If there no arrow on string, play sound
        (Audio|PlaySoundatLocation "/Game/VRWapen/SF_Bow/SF_Bow_sound/SF_half_release.SF_half_release" (Transformation|GetActorLocation) "0, 0, 0" 1.0 1.0 0.0 0 0 0)))))

(fn ConstructionScript)